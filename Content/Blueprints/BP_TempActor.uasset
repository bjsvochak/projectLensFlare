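; BP_TempActor is a test actor with a sphere that gets a random red or blue team material and periodically jumps around.
; The construction script rolls TeamIndex and sets the material.
; A looping BeginPlay timer calls ChooseRandomLocation every ten seconds, doing a swept move to random coordinates, re-rolled separately from the stored NewRandomLocation.
; Move and MoveToLocation offer forward and stored-target movement, but their timers are disconnected.
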(event EventBeginPlay
  (Utilities|Time|SetTimerbyFunctionName 0 "ChooseRandomLocation" 1e+01 true))

(event EventActorBeginOverlap
  (params (OtherActor :type Actor%20Object%20Reference)))

(event EventTick
  (params (DeltaSeconds :type Float%20%28single-precision%29)))

(fn ConstructionScript
  (bind _output_get (Variables|Default|SetTeam%20Index (Math|Random|RandomIntegerinRange 1 2)))
  (if (!= _output_get 0)
    (if (!= _output_get 1)
      ;[1 1 1] Blue Team if team index is not 1
      (Rendering|Material|SetMaterial (Variables|Default|GetSphere) 0 "/Game/Materials/M_Blue_PlayerShip.M_Blue_PlayerShip")
      (else
        ;[1 1 1] Red Team if team index is 1
        (Rendering|Material|SetMaterial (Variables|Default|GetSphere) 0 "/Game/Materials/M_Red_PlayerShip.M_Red_PlayerShip")))))

(fn ChooseRandomLocation
  (bind _returnvalue (Math|Random|RandomFloatinRange -5e+03 5e+03))
  (bind _returnvalue_2 (Math|Random|RandomFloatinRange -5e+03 5e+03))
  (bind _returnvalue_3 (Math|Random|RandomFloatinRange -2e+02 2e+02))
  (bind _returnvalue_4 (Math|Vector|MakeVector _returnvalue_2 _returnvalue_3 _returnvalue))
  (Variables|Default|Setnew%20random%20location _returnvalue_4)
  (Transformation|SetActorLocation _returnvalue_4 true false))

(fn MovetoLocation
  (Transformation|SetActorLocation (Variables|Default|Getnew%20random%20location) true false))

(fn Move
  (Transformation|AddActorLocalOffset (Math|Vector|MakeVector (* (Utilities|Time|GetWorldDeltaSeconds) 1e+03) 0.0 0.0) true false))