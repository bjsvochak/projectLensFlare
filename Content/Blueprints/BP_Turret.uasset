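; BP_Turret is a team-colored turret built from a chassis mesh and a barrel mesh.
; On BeginPlay it creates muzzles from the socketed barrel mesh and registers the chassis mesh through SetChassis.
; The construction script switches on the team enum to apply the blue or red material to both meshes.
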(event EventBeginPlay
  (Class|Turret|CreateMuzzlesfromSocketedMesh (Variables|Default|GetBarrellMesh))
  (Class|Turret|SetChassis (Variables|Default|GetChassisMesh)))

(event EventActorBeginOverlap
  (params (OtherActor :type Actor%20Object%20Reference)))

(event EventTick
  (params (DeltaSeconds :type Float%20%28single-precision%29)))

(fn ConstructionScript
  (bind _chassismesh (Variables|Default|GetChassisMesh))
  (switch Utilities|FlowControl|Switch|SwitchonETeamEnum (Variables|Default|Gete_team)
    (:Team_Blue
      (Rendering|Material|SetMaterial _chassismesh 0 (Variables|Default|GetBlue%20Material)))
    (:Team_Red
      (Rendering|Material|SetMaterial _chassismesh 0 (Variables|Default|GetRed%20Material)))))