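; BP_DreadnoughtFleet is a fleet actor that moves its scene component along a spline.
; Each Tick advances it at the fleet speed, clamped to the current segment's distance goal, then sweeps it to the spline's location and rotation.
; An unconnected chain would spawn blue-team autocannon turrets on carrier, battleship and destroyer sockets and divide the spline into equal goals.
; BeginPlay is empty, so that setup never runs.
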(event EventTick
  (params (DeltaSeconds :type Float%20%28single-precision%29))
  (bind _spline (Variables|Default|GetSpline))
  (bind _output_get (Variables|Default|SetFleet%20Position%20on%20Spline (Math|Float|Clamp(Float) (+ (* DeltaSeconds (Variables|Default|GetFleet%20Move%20Speed)) (Variables|Default|GetFleet%20Position%20on%20Spline)) 0.0 (Utilities|Array|Get(acopy) (Variables|Default|GetFleet%20Distance%20Goals) (Variables|Default|GetFleet%20Current%20Segment)))))
  (Transformation|SetWorldLocationAndRotation (Variables|Default|GetScene) (Spline|GetLocationatDistanceAlongSpline _spline _output_get "World") (Spline|GetRotationatDistanceAlongSpline _spline _output_get "World") true false))

(event EventBeginPlay)

(fn ConstructionScript)