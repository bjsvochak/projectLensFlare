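; Battleship actor that moves its static mesh along a spline in stages, halting at the end of the current segment.
; BeginPlay enables input and splits the spline length into equal cumulative distance goals.
; Tick advances distance at MovementSpeed, clamped to the current goal, and sets mesh location and rotation with sweep.
; Segment advancement is currently unwired, marked for replacement by an enemy capital ship destroyed event.
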(event EventTick
  (params (DeltaSeconds :type Float%20%28single-precision%29))
  (bind _spline (Variables|Components|GetSpline))
  (bind _output_get (Variables|Default|SetCurrent%20Position%20On%20Spline (Math|Float|Clamp(Float) (+ (* DeltaSeconds (Variables|Default|GetMovement%20Speed)) (Variables|Default|GetCurrent%20Position%20On%20Spline)) 0.0 (Utilities|Array|Get(acopy) (Variables|Default|GetSegment%20Distance%20Goals) (Variables|Default|GetCurrent%20Segment%20Number)))))
  (Transformation|SetWorldLocationAndRotation (Variables|Components|GetStaticMesh) (Spline|GetLocationatDistanceAlongSpline _spline _output_get "World") (Spline|GetRotationatDistanceAlongSpline _spline _output_get "World") true false))

(event EventBeginPlay
  (bind _number_of_segments (Variables|Default|GetNumber%20of%20Segments))
  (Input|EnableInput (Game|GetPlayerController 0))
  (for _index (range 1 _number_of_segments)
    (Utilities|Array|Add (Variables|Default|GetSegment%20Distance%20Goals) (* _index (/ (Spline|GetSplineLength (Variables|Components|GetSpline)) (Math|Conversions|ToFloat(Integer) _number_of_segments))))))

(event Input|KeyboardEvents|I
  (params (Key :type Key%20Structure :default "AnyKey"))
  ;[1 1 1] Will be replaced by custom event for when enemy capital ship is destroyed
)

(fn ConstructionScript)