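; BP_SpaceStation is a team-colored space station with Top and Bottom components that spin continuously.
; The construction script swaps both parts' first material by TeamIndex: zero keeps the defaults, values above one use blue, and any other value uses red.
; Tick adds RotationSpeed as local yaw to both parts in the same direction, unscaled by delta time, so spin rate follows frame rate.
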(event EventBeginPlay)

(event EventActorBeginOverlap
  (params (OtherActor :type Actor%20Object%20Reference)))

(event EventTick
  (params (DeltaSeconds :type Float%20%28single-precision%29))
  (bind _rotation_speed (Variables|Default|GetRotation%20Speed))
  (bind _returnvalue (Math|Rotator|MakeRotator 0.0 0.0 _rotation_speed))
  (Transformation|AddLocalRotation (Variables|Default|GetTop) _returnvalue false false)
  (Transformation|AddLocalRotation (Variables|Default|GetBottom) _returnvalue false false))

(fn ConstructionScript
  (bind _team_index (Variables|Default|GetTeam%20Index))
  (bind _top (Variables|Default|GetTop))
  (bind _bottom (Variables|Default|GetBottom))
  (if (not (== _team_index 0))
    (if (> _team_index 1)
      (Rendering|Material|SetMaterial _top 0 "/Game/Materials/M_Blue_SpaceStation.M_Blue_SpaceStation")
      (Rendering|Material|SetMaterial _bottom 0 "/Game/Materials/M_Blue_SpaceStation.M_Blue_SpaceStation")
      (else
        (Rendering|Material|SetMaterial _top 0 "/Game/Materials/M_Red_SpaceStation.M_Red_SpaceStation")
        (Rendering|Material|SetMaterial _bottom 0 "/Game/Materials/M_Red_SpaceStation.M_Red_SpaceStation")))))