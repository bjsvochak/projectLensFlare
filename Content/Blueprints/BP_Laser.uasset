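; BP_Laser is a projectile that damages any BP_PlayerShip it hits and then destroys itself.
; Tick moves it forward along local X at LaserSpeed with a swept offset.
; BeginPlay sets its lifespan and, for a non-zero team index on the referenced PlayerShip, sets the laser mesh material.
; Hits on other actor types are ignored.
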(event EventBeginPlay
  (bind _playership (Variables|Default|GetPlayerShip))
  (bind _lasermesh (Variables|Default|GetLaserMesh))
  (bind _team_index (Variables|/Game/Blueprints/BP_PlayerShip.BP_PlayerShip_C|GetTeam%20Index _playership))
  (Actor|SetLifeSpan (Variables|Default|GetLaser%20Life%20Span))
  (if (!= _team_index 0)
    (if (!= _team_index 1)
      (Rendering|Material|SetMaterial _lasermesh 0 0)
      (else
        (Rendering|Material|SetMaterial _lasermesh 0 0)))))

(event EventTick
  (params (DeltaSeconds :type Float%20%28single-precision%29))
  (Transformation|AddActorLocalOffset (* (* "1.000000, 0, 0" (Variables|Default|GetLaser%20Speed)) DeltaSeconds) true false))

(event Collision|EventHit
  (params (MyComp :type Primitive%20Component%20Object%20Reference) (Other :type Actor%20Object%20Reference) (OtherComp :type Primitive%20Component%20Object%20Reference) (bSelfMoved :type Boolean) (HitLocation :type Vector :default "0, 0, 0") (HitNormal :type Vector :default "0, 0, 0") (NormalImpulse :type Vector :default "0, 0, 0") (Hit :type Hit%20Result%20Structure%20%28by%20ref%29))
  (bind _asbp_player_ship (Utilities|Casting|CastToBP_PlayerShip Other))
  (Default|TakeDamage _asbp_player_ship (Variables|Default|GetDamage%20Amount))
  (Actor|DestroyActor))

(fn ConstructionScript)