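; BP_Destroyer is an actor that moves its static mesh along a spline, stopping at segment boundaries.
; BeginPlay enables player input and splits the spline length into equal cumulative distance goals.
; Tick advances the distance by movement speed, clamps it to the current segment's goal, and sweeps the mesh to that location and rotation.
; The logic that increments the segment number is unconnected, so nothing here moves it to later segments.
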(event EventBeginPlay
  (bind _number_of_segments (Variables|Default|GetNumber%20of%20Segments))
  (Input|EnableInput (Game|GetPlayerController 0))
  (for _index (range 1 _number_of_segments)
    (Utilities|Array|Add (Variables|Default|GetSegment%20Distance%20Goals) (* _index (/ (Spline|GetSplineLength (Variables|Default|GetSpline)) (Math|Conversions|ToFloat(Integer) _number_of_segments))))))

(event EventTick
  (params (DeltaSeconds :type Float%20%28single-precision%29))
  (bind _spline (Variables|Default|GetSpline))
  (bind _output_get (Variables|Default|SetCurrent%20Position%20on%20Spline (Math|Float|Clamp(Float) (+ (* DeltaSeconds (Variables|Default|GetMovement%20Speed)) (Variables|Default|GetCurrent%20Position%20on%20Spline)) 0.0 (Utilities|Array|Get(acopy) (Variables|Default|GetSegment%20Distance%20Goals) (Variables|Default|GetCurrent%20Segment%20Number)))))
  (Transformation|SetWorldLocationAndRotation (Variables|Default|GetStaticMesh) (Spline|GetLocationatDistanceAlongSpline _spline _output_get "World") (Spline|GetRotationatDistanceAlongSpline _spline _output_get "World") true false))

(event Input|KeyboardEvents|O
  (params (Key :type Key%20Structure :default "AnyKey")))

(fn ConstructionScript)